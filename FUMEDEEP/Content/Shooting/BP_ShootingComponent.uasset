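; Actor component that holds a list of BP_Gun actors and fires their bullets toward where the camera is aiming.
; AddGun spawns a BP_Gun with its bullet, fire-rate, burst and damage settings and returns its index in the list.
; Shoot asks the indexed gun whether it can fire, then traces from the camera.
; The bullet spawns at the muzzle rotated toward the hit, or a far forward point on a miss.
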(fn `Add Gun`
  (params (BulletType :type "/Game/Shooting/BP_Bullet Class Reference") (BulletSpeed :type "Float (double-precision)") (FireSpeed :type "Float (double-precision)") (`Burst Bullet Amount` :type Integer) (`Burst Cooldown` :type "Float (double-precision)") (`Gun Damage` :type "Float (double-precision)"))
  (returns (CreatedGun :type Integer))
  (bind _returnvalue (`|SpawnActorFromClass` "/Game/Shooting/BP_Gun.BP_Gun_C" (`KismetMathLibrary.MakeTransform` (0.0 0.0 0.0)) "Undefined" "OverrideRootScale" null BulletType BulletSpeed FireSpeed `Burst Bullet Amount` `Burst Cooldown` `Gun Damage` null))
  (bind _returnvalue_2 (`KismetArrayLibrary.Array_Add` (`self.Guns`) _returnvalue))
  (return _returnvalue_2))

(fn `Shoot`
  (params (Gun :type Integer) (`Start Position` :type "Vector Structure") (Camera :type "CameraComponent Object Reference"))
  (bind _returnvalue (`SceneComponent.K2_GetComponentLocation` Camera))
  (bind _output (`|GetArrayItem` (`self.Guns`) Gun))
  (bind _bullettype (`/Game/Shooting/BP_Gun.BulletType` _output))
  (bind _gun_damage (`/Game/Shooting/BP_Gun.Gun Damage` (`|GetArrayItem` (`self.Guns`) Gun)))
  (bind _returnvalue_2 (`KismetMathLibrary.MakeTransform` `Start Position` (`KismetMathLibrary.Conv_VectorToRotator` (`KismetMathLibrary.GetDirectionUnitVector` `Start Position` (+ (* (`KismetMathLibrary.GetForwardVector` (`SceneComponent.K2_GetComponentRotation` Camera)) 5000.0) (`SceneComponent.K2_GetComponentLocation` Camera))))))
  ;[1 1 1] check if the gun should shoot
  (bind _canshoot (`/Game/Shooting/BP_Gun.HandleShooting` _output))
  (if _canshoot
    ;[1 1 1] raycast to find direction from gun point to objects in front of player
    (bind (_outhit _returnvalue_3) (`KismetSystemLibrary.LineTraceSingle` _returnvalue (+ _returnvalue (* (`KismetMathLibrary.GetForwardVector` (`SceneComponent.K2_GetComponentRotation` Camera)) 1500.0)) "TraceTypeQuery1"))
    (if _returnvalue_3
      (bind _returnvalue_4 (`KismetMathLibrary.MakeTransform` `Start Position` (`KismetMathLibrary.Conv_VectorToRotator` (`KismetMathLibrary.GetDirectionUnitVector` `Start Position` (`.Location` (`GameplayStatics.BreakHitResult` _outhit))))))
      ;[1 1 1] spawn bullet
      (`|SpawnActorFromClass` _bullettype _returnvalue_4 "Undefined" "OverrideRootScale" null _returnvalue_4 _gun_damage null)
      (else
        ;[1 1 1] spawn bullet
        (`|SpawnActorFromClass` _bullettype _returnvalue_2 "Undefined" "OverrideRootScale" null _returnvalue_2 _gun_damage null)))))