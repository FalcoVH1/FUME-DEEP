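; BP_Bullet is a projectile actor that moves via ProjectileMovement and destroys itself once its tick-accumulated timer exceeds Lifetime.
; Construction applies a StartTransform to the actor, and BeginPlay deactivates the GunHit effect.
; Destroy activates GunHit, halts movement and sets Lifetime to one second without resetting the timer, leaving removal to Tick.
; Sphere hit and overlap events are empty, and nothing here calls Destroy.
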(event `self.ReceiveBeginPlay`
  (`ActorComponent.Deactivate` (`self.GunHit`)))

(event `self.ReceiveTick`
  (params (DeltaSeconds :type "Float (single-precision)"))
  (bind _output_get (set `self.LifetimeTimer` (+ DeltaSeconds (`self.LifetimeTimer`))))
  (if (> _output_get (`self.Lifetime`))
    (`self.K2_DestroyActor`)))

(event `self.Sphere.OnComponentHit`
  (params (HitComponent :type "PrimitiveComponent Object Reference") (OtherActor :type "Actor Object Reference") (OtherComp :type "PrimitiveComponent Object Reference") (NormalImpulse :type "Vector Structure") (Hit :type "HitResult Structure (by ref)")))

(event `self.Sphere.OnComponentBeginOverlap`
  (params (OverlappedComponent :type "PrimitiveComponent Object Reference") (OtherActor :type "Actor Object Reference") (OtherComp :type "PrimitiveComponent Object Reference") (OtherBodyIndex :type Integer) (bFromSweep :type Boolean) (SweepResult :type "HitResult Structure (by ref)")))

(fn `Destroy`
  (bind _projectilemovement (`self.ProjectileMovement`))
  (`ActorComponent.Activate` (`self.GunHit`) true)
  (set `MovementComponent.Velocity` (0.0 0.0 0.0) _projectilemovement)
  (set `ProjectileMovementComponent.MaxSpeed` 0.0 _projectilemovement)
  (set `ProjectileMovementComponent.InitialSpeed` 0.0 _projectilemovement)
  (set `self.Lifetime` 1.0))

(fn `UserConstructionScript`
  (bind _output_get (set `self.StartTransform` (`self.StartTransform`)))
  (`self.K2_SetActorTransform` self _output_get false true))