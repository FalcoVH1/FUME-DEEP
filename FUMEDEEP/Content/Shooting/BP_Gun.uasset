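; BP_Gun is a gun Blueprint that provides fire-rate timing, with no projectile or damage logic of its own.
; Tick caches the frame's delta time, which HandleShooting adds to BulletTimer on each call.
; When the timer exceeds FireSpeed, which acts as the interval between shots, HandleShooting subtracts that interval and returns true, carrying over the remainder; otherwise it returns false.
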(event `self.ReceiveTick`
  (params (DeltaSeconds :type "Float (single-precision)"))
  (set `self.DeltaTime` DeltaSeconds))

(fn `HandleShooting`
  (returns (CanShoot :type Boolean))
  (bind _output_get (set `self.Bullet Timer` (+ (`self.Bullet Timer`) (`self.DeltaTime`))))
  (if (> _output_get (`self.FireSpeed`))
    (set `self.Bullet Timer` (- (`self.Bullet Timer`) (`self.FireSpeed`)))
    (return true)
    (else
      (return false))))

(fn `UserConstructionScript`)