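; BP_Mushroom is a bounce pad that launches the player when they overlap its Box trigger.
; The overlap casts to BP_Player and calls LaunchCharacter, overriding existing velocity on all axes.
; Horizontal push follows the Cube's up vector scaled by ForwardBoost, so its tilt steers the bounce, while HeightBoost alone sets vertical speed.
; An unused launch variant adding player forward momentum, a debug print and a no-op branch remain.
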(event `self.Box.OnComponentBeginOverlap`
  (params (OverlappedComponent :type "PrimitiveComponent Object Reference") (OtherActor :type "Actor Object Reference") (OtherComp :type "PrimitiveComponent Object Reference") (OtherBodyIndex :type Integer) (bFromSweep :type Boolean) (SweepResult :type "HitResult Structure (by ref)"))
  (bind _forwardboost (`self.ForwardBoost`))
  (bind (_returnvalue_x _returnvalue_y) (`KismetMathLibrary.BreakVector` (`SceneComponent.GetUpVector` (`self.Cube`))))
  (bind _asbp_player (cast `/Game/Player/BP_Player` OtherActor))
  (if true
    _
    (else
      _))
  (`Character.LaunchCharacter` _asbp_player (`KismetMathLibrary.MakeVector` (* _returnvalue_x _forwardboost) (* _returnvalue_y _forwardboost) (`self.HeightBoost`)) true true))

(fn `UserConstructionScript`)