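; Cannon projectile that plants a BP_Mushroom when its sphere overlaps an actor tagged GROUND.
; The mushroom spawns at the closest collision point on the hit component, using that component's rotation.
; Its forward and height boosts derive from the spawned roll, with thresholds snapping them to fixed values.
; The height boost is only recalculated when the forward check lands in its low or high band, not between.
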(event `self.Sphere1.OnComponentBeginOverlap`
  (params (OverlappedComponent :type "PrimitiveComponent Object Reference") (OtherActor :type "Actor Object Reference") (OtherComp :type "PrimitiveComponent Object Reference") (OtherBodyIndex :type Integer) (bFromSweep :type Boolean) (SweepResult :type "HitResult Structure (by ref)"))
  (if (`self.ActorHasTag` OtherActor "GROUND")
    (bind _returnvalue (`|SpawnActorFromClass` "/Game/BP_Mushroom.BP_Mushroom_C" (`KismetMathLibrary.MakeTransform` (`PrimitiveComponent.GetClosestPointOnCollision` OtherComp (`SceneComponent.K2_GetComponentLocation` (`self.Sphere1`)) "None") (`SceneComponent.K2_GetComponentRotation` OtherComp)) "Undefined" "OverrideRootScale" null null))
    (bind _returnvalue_roll (`KismetMathLibrary.BreakRotator` (`self.K2_GetActorRotation` _returnvalue)))
    (bind _returnvalue_2 (`KismetMathLibrary.Abs` (* _returnvalue_roll (`/Game/BP_Mushroom.ForwardBoost` _returnvalue))))
    (set `/Game/BP_Mushroom.ForwardBoost` (- 10000.0 _returnvalue_2) _returnvalue)
    (if (<= _returnvalue_2 2500.0)
      (set `/Game/BP_Mushroom.ForwardBoost` 0.0 _returnvalue)
      (bind _heightboost (`/Game/BP_Mushroom.HeightBoost` _returnvalue))
      (set `/Game/BP_Mushroom.HeightBoost` (- 10000.0 (`KismetMathLibrary.Abs` (* _returnvalue_roll _heightboost))) _returnvalue :!label _label)
      (if (>= _heightboost 6000.0)
        (set `/Game/BP_Mushroom.HeightBoost` 2500.0 _returnvalue))
      (elif (>= _returnvalue_2 6000.0)
        (set `/Game/BP_Mushroom.ForwardBoost` 8000.0 _returnvalue)
        (goto _label)))))

(fn `UserConstructionScript`)