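; BP_ArmCannon is a player arm cannon that fires BP_CannonProjectile actors toward an aim point.
; Tick accumulates a shot timer, and the Shoot override calls its parent, then fires only once the timer exceeds the shot delay, resetting it.
; The Left flag selects one of two muzzle points, and the projectile spawns there rotated toward the aim end point.
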(event `self.ReceiveTick`
  (params (DeltaSeconds :type "Float (single-precision)"))
  (`parent.ReceiveTick` DeltaSeconds)
  (set `self.ShotTimer` (+ (`self.ShotTimer`) DeltaSeconds)))

(fn `Shoot`
  (params (AimEndPoint :type "Vector Structure"))
  (locals (gunPointPos :type "Vector Structure"))
  (`parent.Shoot` AimEndPoint)
  (if (> (`self.ShotTimer`) (`self.ShotDelay`))
    (set `self.ShotTimer` 0.0)
    (`|ExecutionSequence`
      (:`then_0`
        (if (`self.Left`)
          (set `local.gunPointPos` (`SceneComponent.K2_GetComponentLocation` (`self.GunPoint1`)))
          (else
            (set `local.gunPointPos` (`SceneComponent.K2_GetComponentLocation` (`self.GunPoint`))))))
      (:`then_1`
        (`|SpawnActorFromClass` "/Game/Player/BP_CannonProjectile.BP_CannonProjectile_C" (`KismetMathLibrary.MakeTransform` (`local.gunPointPos`) (`KismetMathLibrary.Conv_VectorToRotator` (`KismetMathLibrary.GetDirectionUnitVector` (`local.gunPointPos`) AimEndPoint))) "Undefined" "OverrideRootScale" null null)))))

(fn `UserConstructionScript`
  (`parent.UserConstructionScript`))