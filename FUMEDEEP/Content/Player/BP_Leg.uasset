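; BP_Leg is a procedurally animated leg with a root and knee joint that swings while the player character moves.
; Each tick it checks player velocity, holding a resting pose with a bent knee when stationary.
; When moving, a speed-scaled timer drives a sine swing on the root and an absolute-value bend on the knee, scaled by Strength.
; An initial Offset shifts each instance's phase.
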(event `self.ReceiveBeginPlay`
  (set `self.timer` (+ (`self.timer`) (`self.offset`))))

(event `self.ReceiveTick`
  (params (DeltaSeconds :type "Float (single-precision)"))
  (bind _returnvalue (`KismetMathLibrary.VSize` (`self.GetVelocity` (`GameplayStatics.GetPlayerCharacter` 0))))
  (if (> _returnvalue 0.0)
    (set `self.State` 1)
    (else
      (set `self.State` 0)))
  (switch `int` (`self.State`)
    (:`0`
      (`SceneComponent.K2_SetRelativeRotation` (`self.LegRoot`) (`KismetMathLibrary.MakeRotator` 0.0) false false)
      (`SceneComponent.K2_SetRelativeRotation` (`self.KneeJoint`) (`KismetMathLibrary.MakeRotator` 0.0 20.0) false false))
    (:`1`
      (bind _output_get (set `self.timer` (+ (`self.timer`) (* DeltaSeconds (/ _returnvalue 10.0)))))
      (bind _output_get_2 (set `self.slerp` (`KismetMathLibrary.DegSin` _output_get)))
      (`SceneComponent.K2_SetRelativeRotation` (`self.LegRoot`) (`KismetMathLibrary.MakeRotator` 0.0 (* _output_get_2 (`self.strength`))) false false)
      (`SceneComponent.K2_SetRelativeRotation` (`self.KneeJoint`) (`KismetMathLibrary.MakeRotator` 0.0 (* (`KismetMathLibrary.Abs` (+ (* _output_get_2 -1.0) 0.5)) (`self.strength`))) false false))))

(fn `UserConstructionScript`)